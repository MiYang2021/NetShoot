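; MyFlyObject is a flying target actor that awards score to the player who shoots it.
; On BeginPlay a timeline drives its absolute world location.
; On damage, the authority waits briefly, then increments the instigator's MyPlayerState score twice.
; It then asks MyGameMode to respawn player 0's controller, regardless of who dealt the damage.
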(event `self.ReceiveAnyDamage`
  (params (Damage :type "Float (single-precision)") (DamageType :type "DamageType Object Reference") (InstigatedBy :type "Controller Object Reference") (DamageCauser :type "Actor Object Reference"))
  ;[1 1 1] 射击加分
  (`/Engine/EditorBlueprintResources/ActorMacros.Switch Has Authority`
    (:`Authority`
      (`KismetSystemLibrary.Delay` 0.2)
      (bind _asmy_player_state (cast `/Game/Blueprints/MyPlayerState` (`Controller.PlayerState` InstigatedBy))
        (:`then`
          (`/Game/Blueprints/MyPlayerState.IncrementScore` _asmy_player_state)
          (`/Game/Blueprints/MyPlayerState.IncrementScore` _asmy_player_state))
        (:`CastFailed`
          _))
      (bind _asmy_game_mode (cast `/Game/Blueprints/MyGameMode` (`GameplayStatics.GetGameMode`)))
      (bind `_as玩家控制器` (cast `PlayerController` (`Pawn.GetController` (`GameplayStatics.GetPlayerPawn` 0))))
      (`/Game/Blueprints/MyGameMode.RespawnPlayerEvent` _asmy_game_mode `_as玩家控制器`))))

(event `self.ReceiveBeginPlay`
  ;[1 1 1] 飞行
  (bind (_direction _move) (`Timeline|时间轴_0`)
    (:`Update`
      (`SceneComponent.K2_SetWorldLocation` (`self.MyFlyObject`) _move false false))))

(fn `UserConstructionScript`)